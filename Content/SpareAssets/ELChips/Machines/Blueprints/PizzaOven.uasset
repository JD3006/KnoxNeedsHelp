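; VR pizza oven machine that advances a Dough through its cooking and roller stages.
; Server-side overlaps track stage 4 dough at the oven and stage 5 at the roller; Tick snaps it in place with physics off when not held.
; A VRPawn touching the button nudges the Cube, starts smoke and cooks stage 4 to 5.
; The roller advances 5 to 6, but is processed only while the oven slot is empty.
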(event `self.ReceiveTick`
  (params (DeltaSeconds :type "Float (single-precision)"))
  (bind _pizzaovenspot1 (`self.PizzaOvenSpot1`))
  (if (`self.isOver`)
    (bind _asdough (cast `/Game/SpareAssets/ELChips/Food/Dough` (`self.objectInside`)))
    (if (not (`/Game/SpareAssets/ELChips/Food/Dough.isBeingHeld` _asdough))
      (bind _staticmesh (`/Game/SpareAssets/ELChips/Food/Dough.StaticMesh` _asdough))
      (`SceneComponent.K2_SetWorldLocation` _staticmesh (`SceneComponent.K2_GetComponentLocation` (`self.PizzaOvenSpot`)) false false)
      (`SceneComponent.K2_SetWorldRotation` :`self` _staticmesh)
      (`PrimitiveComponent.SetSimulatePhysics` _staticmesh false))
    (elif (`self.isOver2`)
      (bind _asdough_2 (cast `/Game/SpareAssets/ELChips/Food/Dough` (`self.objectInsideRoller`)))
      (if (not (`/Game/SpareAssets/ELChips/Food/Dough.isBeingHeld` _asdough_2))
        (bind _staticmesh_2 (`/Game/SpareAssets/ELChips/Food/Dough.StaticMesh` _asdough_2))
        (`SceneComponent.K2_SetWorldLocation` _staticmesh_2 (`SceneComponent.K2_GetComponentLocation` _pizzaovenspot1) false false)
        (`SceneComponent.K2_SetWorldRotation` _staticmesh_2 (`SceneComponent.K2_GetComponentRotation` _pizzaovenspot1) false false)
        (`PrimitiveComponent.SetSimulatePhysics` _staticmesh_2 false)
        (if (== (`/Game/SpareAssets/ELChips/Food/Dough.stage` _asdough_2) 5)
          (`/Game/SpareAssets/ELChips/Food/Dough.updateStage` _asdough_2 6))))))

(event `self.PizzaOvenPlacer.OnComponentBeginOverlap`
  (params (OverlappedComponent :type "PrimitiveComponent Object Reference") (OtherActor :type "Actor Object Reference") (OtherComp :type "PrimitiveComponent Object Reference") (OtherBodyIndex :type Integer) (bFromSweep :type Boolean) (SweepResult :type "HitResult Structure (by ref)"))
  (`/Engine/EditorBlueprintResources/ActorMacros.Switch Has Authority`
    (:`Authority`
      (bind _asdough (cast `/Game/SpareAssets/ELChips/Food/Dough` OtherActor))
      (if (== (`/Game/SpareAssets/ELChips/Food/Dough.stage` _asdough) 4)
        (set `self.isOver` true)
        (set `self.objectInside` _asdough)))))

(event `self.PizzaOvenPlacer.OnComponentEndOverlap`
  (params (OverlappedComponent :type "PrimitiveComponent Object Reference") (OtherActor :type "Actor Object Reference") (OtherComp :type "PrimitiveComponent Object Reference") (OtherBodyIndex :type Integer))
  (`/Engine/EditorBlueprintResources/ActorMacros.Switch Has Authority`
    (:`Authority`
      (if (== OtherActor (`self.objectInside`))
        (set `self.isOver` false)
        (set `self.objectInside` null)))))

(event `self.PizzaOvenButton.OnComponentBeginOverlap`
  (params (OverlappedComponent :type "PrimitiveComponent Object Reference") (OtherActor :type "Actor Object Reference") (OtherComp :type "PrimitiveComponent Object Reference") (OtherBodyIndex :type Integer) (bFromSweep :type Boolean) (SweepResult :type "HitResult Structure (by ref)"))
  (bind _cube (`self.Cube`))
  (bind (_returnvalue_location _returnvalue_rotation) (`KismetMathLibrary.BreakTransform` (`SceneComponent.GetRelativeTransform` _cube)))
  (bind (_returnvalue_location_2 _returnvalue_rotation_2) (`KismetMathLibrary.BreakTransform` (`SceneComponent.GetRelativeTransform` _cube)))
  (cast `/Game/VRTemplate/Blueprints/VRPawn` OtherActor)
  (bind _asdough (cast `/Game/SpareAssets/ELChips/Food/Dough` (`self.objectInside`)))
  (if (`/Game/SpareAssets/ELChips/Food/Dough.isBeingHeld` _asdough)
    _
    (elif (== (`/Game/SpareAssets/ELChips/Food/Dough.stage` _asdough) 4)
      (`KismetSystemLibrary.MoveComponentTo` _cube (+ _returnvalue_location_2 (0.0 3.0 0.0)) _returnvalue_rotation_2 false false 0.1)
      (`ActorComponent.Activate` (`self.SmokeCook`) true)
      (`/Game/SpareAssets/ELChips/Food/Dough.updateStage` _asdough 5)
      (`KismetSystemLibrary.MoveComponentTo` _cube (+ _returnvalue_location (0.0 -3.0 0.0)) _returnvalue_rotation false false 0.1))))

(event `self.PizzaRollerPlacer.OnComponentBeginOverlap`
  (params (OverlappedComponent :type "PrimitiveComponent Object Reference") (OtherActor :type "Actor Object Reference") (OtherComp :type "PrimitiveComponent Object Reference") (OtherBodyIndex :type Integer) (bFromSweep :type Boolean) (SweepResult :type "HitResult Structure (by ref)"))
  (`/Engine/EditorBlueprintResources/ActorMacros.Switch Has Authority`
    (:`Authority`
      (bind _asdough (cast `/Game/SpareAssets/ELChips/Food/Dough` OtherActor))
      (if (== (`/Game/SpareAssets/ELChips/Food/Dough.stage` _asdough) 5)
        (set `self.isOver2` true)
        (set `self.objectInsideRoller` _asdough)))))

(event `self.PizzaRollerPlacer.OnComponentEndOverlap`
  (params (OverlappedComponent :type "PrimitiveComponent Object Reference") (OtherActor :type "Actor Object Reference") (OtherComp :type "PrimitiveComponent Object Reference") (OtherBodyIndex :type Integer))
  (`/Engine/EditorBlueprintResources/ActorMacros.Switch Has Authority`
    (:`Authority`
      (if (== OtherActor (`self.objectInsideRoller`))
        (set `self.isOver2` false)
        (set `self.objectInsideRoller` null)))))

(fn `UserConstructionScript`)