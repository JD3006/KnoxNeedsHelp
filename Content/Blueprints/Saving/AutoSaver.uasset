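; AutoSaver is an actor that saves and restores which minigames are unlocked, using the "default" save slot.
; On BeginPlay it asynchronously loads a KNHSaveClass and passes UnlockedMinigames to the MenuConsole actor, or saves and passes an initial unlock string if loading fails.
; Its saveCurrentGame event writes a given unlock value into a fresh save object and saves it asynchronously, overwriting the slot.
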(event `self.ReceiveBeginPlay`
  (bind (_savegame _bsuccess) (`AsyncActionHandleSaveGame.AsyncLoadGameFromSlot` "default")
    (:`Completed`
      (if _bsuccess
        (bind _asknhsave_class (cast `/Game/Blueprints/Saving/KNHSaveClass` _savegame)
          (:`then`
            (bind _returnvalue (`GameplayStatics.GetActorOfClass` "/Game/SpareAssets/ARHub/Terminal/MenuConsole.MenuConsole_C"))
            (`/Game/SpareAssets/ARHub/Terminal/MenuConsole.loadGameSaveTerminal` _returnvalue (`/Game/Blueprints/Saving/KNHSaveClass.unlockedMinigames` _asknhsave_class)))
          (:`CastFailed`
            (`KismetSystemLibrary.PrintText` "uhoh")))
        (else
          (`self.saveCurrentGame` "10000")
          (bind _returnvalue_2 (`GameplayStatics.GetActorOfClass` "/Game/SpareAssets/ARHub/Terminal/MenuConsole.MenuConsole_C"))
          (`/Game/SpareAssets/ARHub/Terminal/MenuConsole.loadGameSaveTerminal` _returnvalue_2 "10000")
          (`KismetSystemLibrary.PrintText` "save slot nonexistent, creating new"))))))

(event `self.ReceiveTick`
  (params (DeltaSeconds :type "Float (single-precision)")))

(event `saveCurrentGame`
  (params (umini :type String))
  (bind _returnvalue (`GameplayStatics.CreateSaveGameObject` "/Game/Blueprints/Saving/KNHSaveClass.KNHSaveClass_C"))
  (bind _output_get (set `self.saveGameObj` _returnvalue))
  (set `/Game/Blueprints/Saving/KNHSaveClass.unlockedMinigames` umini _output_get)
  (`AsyncActionHandleSaveGame.AsyncSaveGameToSlot` _returnvalue "default"))

(fn `UserConstructionScript`)