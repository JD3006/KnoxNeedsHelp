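; SideDishTraySpawner is a dispenser actor that keeps a SideDishBox tray available at its position.
; Tick checks the TraySpawned reference and, when it appears empty, spawns a new box at the StaticMesh's world transform and stores it.
; When that tracked box leaves the Trigger volume, the server clears the reference so a replacement spawns.
; Only the clearing is authority-gated; the Tick spawn has no authority check.
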(event `self.ReceiveBeginPlay`)

(event `self.ReceiveTick`
  (params (DeltaSeconds :type "Float (single-precision)"))
  (if (== (`self.traySpawned`) null)
    (bind _returnvalue (`|SpawnActorFromClass` "/Game/Blueprints/FoodPrep/PickupObjects/SideDishBox.SideDishBox_C" (`SceneComponent.K2_GetComponentToWorld` (`self.StaticMesh`)) "Undefined" "MultiplyWithRoot" null null))
    (set `self.traySpawned` _returnvalue)))

(event `self.Trigger.OnComponentEndOverlap`
  (params (OverlappedComponent :type "PrimitiveComponent Object Reference") (OtherActor :type "Actor Object Reference") (OtherComp :type "PrimitiveComponent Object Reference") (OtherBodyIndex :type Integer))
  (`/Engine/EditorBlueprintResources/ActorMacros.Switch Has Authority`
    (:`Authority`
      (if (== OtherActor (`self.traySpawned`))
        (set `self.traySpawned` null)))))

(fn `UserConstructionScript`)