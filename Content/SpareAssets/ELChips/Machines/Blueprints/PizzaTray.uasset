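; PizzaTray is a tray actor that holds a Dough actor in place when it is released over the tray.
; Box overlap events store the most recent Dough and whether it is over the tray.
; On the server, Tick checks that Dough while unheld: over the tray, it disables physics and pins the mesh just above the tray origin with zeroed rotation.
; Otherwise it re-enables physics.
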(event `self.ReceiveTick`
  (params (DeltaSeconds :type "Float (single-precision)"))
  (bind (_returnvalue_x _returnvalue_y _returnvalue_z) (`KismetMathLibrary.BreakVector` (`self.K2_GetActorLocation`)))
  (bind _dough (`self.dough`))
  (bind _staticmesh (`/Game/SpareAssets/ELChips/Food/Dough.StaticMesh` _dough))
  (`/Engine/EditorBlueprintResources/ActorMacros.Switch Has Authority`
    (:`Authority`
      (if (!= _dough null)
        (if (`/Game/SpareAssets/ELChips/Food/Dough.isBeingHeld` _dough)
          _
          (elif (`self.isOver`)
            (`PrimitiveComponent.SetSimulatePhysics` _staticmesh false)
            (`SceneComponent.K2_SetWorldLocation` _staticmesh (`KismetMathLibrary.MakeVector` _returnvalue_x _returnvalue_y (+ _returnvalue_z 0.5)) false false)
            (`SceneComponent.K2_SetWorldRotation` :`self` _staticmesh)
            (else
              (`PrimitiveComponent.SetSimulatePhysics` _staticmesh true))))))))

(event `self.Box.OnComponentBeginOverlap`
  (params (OverlappedComponent :type "PrimitiveComponent Object Reference") (OtherActor :type "Actor Object Reference") (OtherComp :type "PrimitiveComponent Object Reference") (OtherBodyIndex :type Integer) (bFromSweep :type Boolean) (SweepResult :type "HitResult Structure (by ref)"))
  (bind _asdough (cast `/Game/SpareAssets/ELChips/Food/Dough` OtherActor))
  (set `self.dough` _asdough)
  (set `self.isOver` true))

(event `self.Box.OnComponentEndOverlap`
  (params (OverlappedComponent :type "PrimitiveComponent Object Reference") (OtherActor :type "Actor Object Reference") (OtherComp :type "PrimitiveComponent Object Reference") (OtherBodyIndex :type Integer))
  (bind _asdough (cast `/Game/SpareAssets/ELChips/Food/Dough` OtherActor))
  (set `self.dough` _asdough)
  (set `self.isOver` false))

(fn `UserConstructionScript`)