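; Manager for the food prep game that tracks the game stage and moves players to hard-coded positions when the game starts.
; StartGame advances the stage, plays the FadeBlack sequence on the first LevelSequenceActor found, then teleports pawns after a short delay.
; TeleportAll loops over player controllers, placing the first player's pawn at one position and all others at a second.
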(event `self.ReceiveBeginPlay`
  (set `self.gameStage` 0))

(event `startGame`
  (set `self.gameStage` 1)
  (`self.FadeClients`)
  (`KismetSystemLibrary.Delay` 1.0)
  (`self.teleportAll` (1771.528462 61.08877 105.0) (1771.528462 201.240623 105.0)))

(event `teleportAll`
  (params (Position :type "Vector Structure") (Position2 :type "Vector Structure"))
  (for _index (range (`GameplayStatics.GetNumPlayerControllers`))
    (if (== _index 0)
      (bind _returnvalue (`GameplayStatics.GetPlayerPawn` _index))
      (`self.K2_SetActorLocation` _returnvalue Position false false)
      (else
        (`self.K2_SetActorLocation` _returnvalue Position2 false false)))))

(event `FadeClients`
  (bind _returnvalue (`GameplayStatics.GetActorOfClass` "/Script/LevelSequence.LevelSequenceActor"))
  (`LevelSequenceActor.SetSequence` _returnvalue "/Game/Blueprints/FadeSequences/FadeBlack.FadeBlack")
  (`MovieSceneSequencePlayer.Play` (`LevelSequenceActor.SequencePlayer` _returnvalue)))

(fn `UserConstructionScript`)