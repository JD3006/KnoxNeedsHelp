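; Pretzel vendor machine that keeps one Pretzel and one MeatPretzel stocked at their display spots.
; Tick checks both tracked references and spawns a replacement at the matching spot whenever one is empty.
; Each trigger's end overlap clears its reference on the server when the tracked item leaves, prompting a restock.
; The Tick spawning itself has no authority check.
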(event `self.ReceiveTick`
  (params (DeltaSeconds :type "Float (single-precision)"))
  (`|ExecutionSequence`
    (:`then_0`
      (if (== (`self.pretzelIn`) null)
        (bind _returnvalue (`|SpawnActorFromClass` "/Game/SpareAssets/ELChips/Food/Pretzel.Pretzel_C" (`SceneComponent.K2_GetComponentToWorld` (`self.PretzelSpot`)) "Undefined" "MultiplyWithRoot" null null))
        (set `self.pretzelIn` _returnvalue)))
    (:`then_1`
      (if (== (`self.mpretzelIn`) null)
        (bind _returnvalue_2 (`|SpawnActorFromClass` "/Game/SpareAssets/ELChips/Food/MeatPretzel.MeatPretzel_C" (`SceneComponent.K2_GetComponentToWorld` (`self.MeatPretzelSpot`)) "Undefined" "MultiplyWithRoot" null null))
        (set `self.mpretzelIn` _returnvalue_2)))))

(event `self.PretzelTrigger.OnComponentEndOverlap`
  (params (OverlappedComponent :type "PrimitiveComponent Object Reference") (OtherActor :type "Actor Object Reference") (OtherComp :type "PrimitiveComponent Object Reference") (OtherBodyIndex :type Integer))
  (`/Engine/EditorBlueprintResources/ActorMacros.Switch Has Authority`
    (:`Authority`
      (if (== OtherActor (`self.pretzelIn`))
        (set `self.pretzelIn` null)))))

(event `self.MeatPretzelTrigger.OnComponentEndOverlap`
  (params (OverlappedComponent :type "PrimitiveComponent Object Reference") (OtherActor :type "Actor Object Reference") (OtherComp :type "PrimitiveComponent Object Reference") (OtherBodyIndex :type Integer))
  (`/Engine/EditorBlueprintResources/ActorMacros.Switch Has Authority`
    (:`Authority`
      (if (== OtherActor (`self.mpretzelIn`))
        (set `self.mpretzelIn` null)))))

(fn `UserConstructionScript`)