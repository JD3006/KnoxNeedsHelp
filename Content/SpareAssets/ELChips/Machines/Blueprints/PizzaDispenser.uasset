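; PizzaDispenser is a VR machine that spawns a pizza ingredient when its button is pressed.
; A VRPawn overlapping MeatTrigger runs an authority-only sequence that animates MeatButton in, calls SpawnTopping, then animates it back out.
; The ButtonPressed flag blocks repeat presses until the sequence finishes.
; SpawnTopping handles only type 0, spawning Dough just below the actor despite the Meat naming.
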(event `SpawnTopping`
  (params (toppingType :type Integer))
  (if (== toppingType 0)
    (`|SpawnActorFromClass` "/Game/SpareAssets/ELChips/Food/Dough.Dough_C" (`KismetMathLibrary.MakeTransform` (- (`self.K2_GetActorLocation`) (0.0 0.0 10.0))) "Undefined" "MultiplyWithRoot" null null)))

(event `self.ReceiveBeginPlay`
  (set `self.buttonPressed` false))

(event `self.MeatTrigger.OnComponentBeginOverlap`
  (params (OverlappedComponent :type "PrimitiveComponent Object Reference") (OtherActor :type "Actor Object Reference") (OtherComp :type "PrimitiveComponent Object Reference") (OtherBodyIndex :type Integer) (bFromSweep :type Boolean) (SweepResult :type "HitResult Structure (by ref)"))
  (bind _meatbutton (`self.MeatButton`))
  (bind _meatbutton_2 (`self.MeatButton`))
  (if (not (`self.buttonPressed`))
    (cast `/Game/VRTemplate/Blueprints/VRPawn` OtherActor)
    (`/Engine/EditorBlueprintResources/ActorMacros.Switch Has Authority`
      (:`Authority`
        (set `self.buttonPressed` true)
        (`KismetSystemLibrary.MoveComponentTo` _meatbutton_2 (+ (`SceneComponent.RelativeLocation` _meatbutton_2) (0.0 -5.0 0.0)) (`SceneComponent.RelativeRotation` _meatbutton_2) false false 0.2)
        (`self.SpawnTopping` 0)
        (`KismetSystemLibrary.MoveComponentTo` _meatbutton (+ (`SceneComponent.RelativeLocation` _meatbutton) (0.0 5.0 0.0)) (`SceneComponent.RelativeRotation` _meatbutton) false false 0.2)
        (set `self.buttonPressed` false)))))

(fn `UserConstructionScript`)